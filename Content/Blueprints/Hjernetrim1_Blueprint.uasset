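; Brain-teaser trigger actor (Hjernetrim1) that shows the Puzzle1 UI widget on overlap.
; Each overlap creates and stores a new Puzzle1 widget, adding it to the viewport if PlayerActivate is set and otherwise clearing all widgets.
; Ending the overlap clears all widgets, then re-adds the HUD referenced by the player's TimBlueprint character.
; The overlapping actor is never checked.
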(event EventBeginPlay)

(event Collision|EventActorBeginOverlap
  (params (OtherActor :type Actor%20Object%20Reference))
  (bind _returnvalue (UserInterface|CreateWidget "/Game/Blueprints/Puzzle1.Puzzle1_C"))
  (bind _output_get (Variables|Default|SetPuzzle_Referance _returnvalue))
  (if (Variables|Default|GetPlayerActivate)
    (UserInterface|Viewport|AddtoViewport _output_get 0)
    (else
      (Viewport|RemoveAllWidgets))))

(event EventTick
  (params (DeltaSeconds :type Float%20%28single-precision%29)))

(event Collision|EventActorEndOverlap
  (params (OtherActor :type Actor%20Object%20Reference))
  (Viewport|RemoveAllWidgets)
  (bind _astim_blueprint (Utilities|Casting|CastToTimBlueprint (Game|GetPlayerCharacter 0)))
  (UserInterface|Viewport|AddtoViewport (Variables|/Game/Blueprints/TimBlueprint.TimBlueprint_C|GetHUD%20reference _astim_blueprint) 0))

(fn ConstructionScript)