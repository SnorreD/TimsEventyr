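; Boss encounter actor that shows a boss health bar while the player character Tim overlaps it.
; On begin overlap it creates a BossHealth widget, stores the reference and adds it to the viewport.
; On end overlap it removes the widget, then sets AutoDestroyWhenFinished according to whether the widget's health percent is zero or below.
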(event EventBeginPlay)

(event Collision|EventActorBeginOverlap
  (params (OtherActor :type Actor%20Object%20Reference))
  (Utilities|Casting|CastToTim OtherActor)
  (bind _returnvalue (UserInterface|CreateWidget "/Game/Blueprints/HUD/BossHealth.BossHealth_C"))
  (bind _output_get (Variables|Default|SetHUD_Referance _returnvalue))
  (UserInterface|Viewport|AddtoViewport _output_get 0))

(event Collision|EventActorEndOverlap
  (params (OtherActor :type Actor%20Object%20Reference))
  (bind _hud_referance (Variables|Default|GetHUD_Referance))
  (Utilities|Casting|CastToTim OtherActor)
  (Widget|RemovefromParent _hud_referance)
  (Variables|Default|SetbAutoDestroyWhenFinished (>= 0.0 (Default|GetPercent0 _hud_referance))))

(event EventTick
  (params (DeltaSeconds :type Float%20%28single-precision%29)))

(fn ConstructionScript)