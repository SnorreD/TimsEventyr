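; Last boss Blueprint that sets up hand capsules and triggers a Matinee sequence once the Finished flag is set.
; BeginPlay attaches capsules to the bones behind the hand sockets, though RightHandCapsule is first assigned LeftHandCapsule, so both attachments move the left capsule.
; Tick polls Finished, searches all Matinee actors for the one named MatineeActor69, plays it and clears the flag.
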(event EventBeginPlay
  (bind _skeletalmesh (Variables|Default|GetSkeletalMesh))
  (bind _output_get (Variables|Default|SetRightHandCapsule (Variables|Default|GetLeftHandCapsule)))
  (Transformation|AttachComponentToComponent _output_get _skeletalmesh (Class|SkinnedMeshComponent|GetSocketBoneName _skeletalmesh "SocketRightHand") "KeepRelative" "KeepRelative" "KeepRelative" true)
  (bind _output_get_2 (Variables|Default|SetLeftHandCapsule (Variables|Default|GetLeftHandCapsule)))
  (Transformation|AttachComponentToComponent _output_get_2 _skeletalmesh (Class|SkinnedMeshComponent|GetSocketBoneName _skeletalmesh "SocketLeftHand") "SnapToTarget" "SnapToTarget" "SnapToTarget" true))

(event Collision|EventActorBeginOverlap
  (params (OtherActor :type Actor%20Object%20Reference)))

(event EventTick
  (params (DeltaSeconds :type Float%20%28single-precision%29))
  (if (Variables|Default|GetFinished)
    (bind _outactors (Actor|GetAllActorsOfClass "/Script/Engine.MatineeActor"))
    (for _array_element _outactors
      (if (Utilities|Enum|Equal(Enum) (Utilities|GetObjectName _array_element) "MatineeActor69")
        (Audio|Components|Audio|Play _array_element)
        (Variables|Default|SetFinished false)))
    (if (Utilities|Enum|Equal(Enum) (Utilities|GetObjectName _array_element) "MatineeActor69")
      (Audio|Components|Audio|Play _array_element)
      (Variables|Default|SetFinished false))))

(fn ConstructionScript)